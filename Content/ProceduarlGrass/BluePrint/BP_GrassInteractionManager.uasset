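; BP_GrassInteractionManager is an actor that records a fading trail of the player character's position in a render target for grass interaction.
; At BeginPlay it creates decay, brush and copy materials and publishes the area's fixed center and world size to MPC_GrassInteraction.
; Each Tick applies frame-rate-independent decay from the previous target, stamps the brush at the player, then copies the result back as history.
; Actors tagged GrassInteractor are gathered but not drawn.
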(event EventBeginPlay
  (bind _returnvalue (Rendering|Material|CreateDynamicMaterialInstance "/Game/ProceduarlGrass/Materials/M_RT_Decay.M_RT_Decay" "None" "None" :!class /Script/Engine.KismetMaterialLibrary))
  (Variables|Default|SetMID_Decay%20 _returnvalue)
  (bind _returnvalue_2 (Rendering|Material|CreateDynamicMaterialInstance "/Game/ProceduarlGrass/Materials/M_RT_Brush.M_RT_Brush" "None" "None" :!class /Script/Engine.KismetMaterialLibrary))
  (Variables|Default|SetMID_Brush%20 _returnvalue_2)
  (bind _returnvalue_3 (Rendering|Material|CreateDynamicMaterialInstance "/Game/ProceduarlGrass/Materials/M_RT_Copy.M_RT_Copy" "None" "None" :!class /Script/Engine.KismetMaterialLibrary))
  (Variables|Default|SetMID_Copy _returnvalue_3)
  (bind _outactors (Actor|GetAllActorswithTag "GrassInteractor"))
  (Variables|Default|SetInteractors%20 _outactors)
  (Variables|Default|SetRT_Center%20 (Transformation|GetActorLocation))
  (Rendering|Material|SetVectorParameterValue "/Game/ProceduarlGrass/Materials/MPC_GrassInteraction.MPC_GrassInteraction" "RT_Center" (Math|Conversions|ToLinearColor(Vector) (Variables|Default|GetRT_Center%20)) :!class /Script/Engine.KismetMaterialLibrary)
  (Rendering|Material|SetScalarParameterValue "/Game/ProceduarlGrass/Materials/MPC_GrassInteraction.MPC_GrassInteraction" "RT_WorldSize" (Variables|Default|GetRT_WorldSize%20) :!class /Script/Engine.KismetMaterialLibrary))

(event Collision|EventActorBeginOverlap
  (params (OtherActor :type Actor%20Object%20Reference)))

(event EventTick
  (params (DeltaSeconds :type Float%20%28single-precision%29))
  (bind _returnvalue (Game|GetPlayerCharacter 0))
  (bind _rt_worldsize_ (Variables|Default|GetRT_WorldSize%20))
  (bind _rt_size_ (Variables|Default|GetRT_Size%20))
  (bind _brushpixelsize (Variables|Default|GetBrushPixelSize))
  (bind _mid_decay_ (Variables|Default|GetMID_Decay%20))
  (bind _rt_center_ (Variables|Default|GetRT_Center%20))
  (bind _returnvalue_2 (Transformation|GetActorLocation _returnvalue))
  (bind _returnvalue_3 (* _brushpixelsize 0.5))
  (Variables|Default|SetDecay%20 (Math|Float|Power 0.94 (* DeltaSeconds 6e+01)))
  (Rendering|Material|SetTextureParameterValue _mid_decay_ "PrevRT" "/Game/ProceduarlGrass/Materials/RT_GrassPrev.RT_GrassPrev")
  (Rendering|Material|SetScalarParameterValue _mid_decay_ "Decay" (Variables|Default|GetDecay%20) :!class /Script/Engine.MaterialInstanceDynamic)
  (Rendering|DrawMaterialtoRenderTarget "/Game/ProceduarlGrass/Materials/RT_GrassState.RT_GrassState" _mid_decay_)
  (bind (_canvas _size _context) (Rendering|BeginDrawCanvastoRenderTarget "/Game/ProceduarlGrass/Materials/RT_GrassState.RT_GrassState"))
  (Canvas|DrawMaterial :self _canvas :RenderMaterial (Variables|Default|GetMID_Brush%20) :ScreenPosition (Math|Vector2D|MakeVector2D (- (* (+ (/ (- (.x _returnvalue_2) (.x _rt_center_)) _rt_worldsize_) 0.5) _rt_size_) _returnvalue_3) (- (* (+ (/ (- (.y _returnvalue_2) (.y _rt_center_)) _rt_worldsize_) 0.5) _rt_size_) _returnvalue_3)) :ScreenSize (Math|Vector2D|MakeVector2D _brushpixelsize _brushpixelsize) :CoordinateSize "(X=1.000000,Y=1.000000)" :PivotPoint "(X=0.000000,Y=0.000000)")
  (Rendering|EndDrawCanvastoRenderTarget _context)
  (Rendering|Material|SetTextureParameterValue (Variables|Default|GetMID_Copy) "StateRT" "/Game/ProceduarlGrass/Materials/RT_GrassState.RT_GrassState")
  (Rendering|DrawMaterialtoRenderTarget "/Game/ProceduarlGrass/Materials/RT_GrassPrev.RT_GrassPrev" (Variables|Default|GetMID_Copy)))

(fn ConstructionScript)